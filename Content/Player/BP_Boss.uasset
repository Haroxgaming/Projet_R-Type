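; BP_Boss is a boss that starts firing projectiles once the player enters its Box trigger.
; A looping timer, its interval randomized once, spawns BP_Projectile using random picks among three arrows for position and direction.
; Projectile overlaps on Box1 reduce health and briefly flash the meshes with a hit material.
; At zero health it destroys itself, with a delayed Menu_Map load wired afterward.
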(event OnComponentBeginOverlap(Box)
  (params (OverlappedComponent :type Primitive%20Component%20Object%20Reference) (OtherActor :type Actor%20Object%20Reference) (OtherComp :type Primitive%20Component%20Object%20Reference) (OtherBodyIndex :type Integer) (bFromSweep :type Boolean) (SweepResult :type Hit%20Result%20Structure%20%28by%20ref%29))
  (Utilities|Casting|CastToBP_Player OtherActor)
  (Utilities|FlowControl|DoOnce false
    (:Completed
      (CallFunction|Attack))))

(event OnComponentBeginOverlap(Box1)
  (params (OverlappedComponent :type Primitive%20Component%20Object%20Reference) (OtherActor :type Actor%20Object%20Reference) (OtherComp :type Primitive%20Component%20Object%20Reference) (OtherBodyIndex :type Integer) (bFromSweep :type Boolean) (SweepResult :type Hit%20Result%20Structure%20%28by%20ref%29))
  (Utilities|Casting|CastToBP_Projectile OtherActor)
  (Math|Integer|DecrementInt (Variables|Default|GetHealth)
    (:%20%20
      (Utilities|FlowControl|Sequence
        (:then_0
          (if (<= (Variables|Default|GetHealth) 0)
            (Actor|DestroyActor)
            (Utilities|FlowControl|Delay 0.2)
            (Game|OpenLevel(byObjectReference) "/Game/Player/Menu_Map.Menu_Map")))
        (:then_1
          (Utilities|IsValid self
            (:Is%20Valid
              (Rendering|Material|SetMaterial (Variables|Default|GetCylinder2) 0 "/Game/Player/M_Hit.M_Hit")
              (Utilities|FlowControl|Delay 0.2)
              (Utilities|IsValid self
                (:Is%20Valid
                  (Rendering|Material|SetMaterial (Variables|Default|GetStaticMesh) 0 "/Game/Player/M_Boss_Inst.M_Boss_Inst")
                  (Rendering|Material|SetMaterial (Variables|Default|GetCylinder2) 0 "/Engine/BasicShapes/BasicShapeMaterial.BasicShapeMaterial"))))))))))

(event Custom|Spawn%20Bullet
  (bind _returnvalue (Math|Random|RandomIntegerinRange 0 2))
  (bind _arrow (Variables|Default|GetArrow))
  (bind _arrow1 (Variables|Default|GetArrow1))
  (bind _arrow2 (Variables|Default|GetArrow2))
  (bind _returnvalue_2 (Utilities|Select :Index _returnvalue :Option%200 _arrow :Option%201 _arrow1 :Option%202 _arrow2))
  (Game|SpawnActorfromClass "/Game/BP_Projectile.BP_Projectile_C" (Math|Transform|MakeTransform (Transformation|GetWorldLocation _returnvalue_2) (Math|Conversions|RotationFromXVector (Math|Vector|GetForwardVector _returnvalue_2)) "1.000000,1.000000,1.000000") "AlwaysSpawn" "MultiplyWithRoot" self 1.2e+03 0))

(event Custom|Attack
  (Utilities|Time|SetTimerbyEvent (delegate Custom|Spawn%20Bullet) (Math|Random|RandomFloatinRange 0.2 1.0) true))

(event EventBeginPlay)

(event Collision|EventActorBeginOverlap
  (params (OtherActor :type Actor%20Object%20Reference)))

(event EventTick
  (params (DeltaSeconds :type Float%20%28single-precision%29)))

(fn ConstructionScript)